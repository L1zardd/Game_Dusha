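; Door actor that slides its Cube component vertically to open and close, playing a door sound at its location each time.
; OpenDoor and CloseDoor store the current relative height, set a raised or zero target, and share one Timeline.
; The Timeline restarts from the beginning and linearly eases the height from the stored value to the target, so each move begins at the door's current position.
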(event `OpenDoor`
  (bind (_relativelocation_x _relativelocation_y _relativelocation_z) (`KismetMathLibrary.BreakVector` (`SceneComponent.RelativeLocation` (`self.Cube`))))
  (set `self.CurrewntHeight` _relativelocation_z)
  (set `self.HewHeight` 300.0)
  (`GameplayStatics.PlaySoundAtLocation` "/Game/sound/Effects/Звук_двери_игра.Звук_двери_игра" (`self.K2_GetActorLocation`) (struct) 1.0 1.0 0.0 null null null null :!label _label)
  (bind (_direction _alpha) (`Timeline|Timeline` :!via `PlayFromStart`)
    (:`Update`
      (`SceneComponent.K2_SetRelativeLocation` (`self.Cube`) (`KismetMathLibrary.MakeVector` 0.0 0.0 (`|EaseFunction` "Linear" _alpha (`self.CurrewntHeight`) (`self.HewHeight`))) false false))))

(event `CloseDoor`
  (bind (_relativelocation_x _relativelocation_y _relativelocation_z) (`KismetMathLibrary.BreakVector` (`SceneComponent.RelativeLocation` (`self.Cube`))))
  (set `self.CurrewntHeight` _relativelocation_z)
  (set `self.HewHeight` 0.0)
  (goto _label))

(fn `UserConstructionScript`)