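; Pressure plate actor that opens a linked door while anything overlaps its box and closes it once the box is empty.
; Begin and end overlap events maintain an overlap counter, so only the last exit deactivates the plate.
; Activate and Deactivate are guarded by an IsActive flag, and each plays a sound, swaps the frame material and drives the linked door if valid.
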(event `Activate`
  (bind _linkeddoor (`self.LinkedDoor`))
  (if (not (`self.IsActive`))
    (`GameplayStatics.PlaySoundAtLocation` "/Game/sound/Effects/ButtonSC.ButtonSC" (`self.K2_GetActorLocation`) (struct) 1.0 1.0 0.0 null null null null)
    (set `self.IsActive` true)
    (`PrimitiveComponent.SetMaterial` (`self.Frame`) 0 "/Engine/MapTemplates/Materials/BasicAsset03.BasicAsset03")
    (`/Engine/EditorBlueprintResources/StandardMacros.IsValid` _linkeddoor
      (:`Is Valid`
        (`/Game/blueprints/Door_BP.OpenDoor` _linkeddoor)))))

(event `Deactivate`
  (bind _linkeddoor (`self.LinkedDoor`))
  (if (`self.IsActive`)
    (`GameplayStatics.PlaySoundAtLocation` "/Engine/VREditor/Sounds/UI/Camera_Shutter.Camera_Shutter" (`self.K2_GetActorLocation`) (struct) 1.0 1.0 0.0 null null null null)
    (set `self.IsActive` false)
    (`PrimitiveComponent.SetMaterial` (`self.Frame`) 0 "/Engine/MapTemplates/Materials/BasicAsset02.BasicAsset02")
    (`/Engine/EditorBlueprintResources/StandardMacros.IsValid` _linkeddoor
      (:`Is Valid`
        (`/Game/blueprints/Door_BP.CloseDoor` _linkeddoor)))))

(event `self.Box.OnComponentBeginOverlap`
  (params (OverlappedComponent :type "PrimitiveComponent Object Reference") (OtherActor :type "Actor Object Reference") (OtherComp :type "PrimitiveComponent Object Reference") (OtherBodyIndex :type Integer) (bFromSweep :type Boolean) (SweepResult :type "HitResult Structure (by ref)"))
  (`self.Activate`)
  (`/Engine/EditorBlueprintResources/StandardMacros.IncrementInt` (`self.OverLappedActors`)))

(event `self.Box.OnComponentEndOverlap`
  (params (OverlappedComponent :type "PrimitiveComponent Object Reference") (OtherActor :type "Actor Object Reference") (OtherComp :type "PrimitiveComponent Object Reference") (OtherBodyIndex :type Integer))
  (bind _result (`/Engine/EditorBlueprintResources/StandardMacros.DecrementInt` (`self.OverLappedActors`))
    (:`  `
      (if (== _result 0)
        (`self.Deactivate`)))))

(fn `UserConstructionScript`)