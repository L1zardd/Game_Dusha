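; BpThunder1 is a thunder projectile with flipbook visuals that damages what it hits.
; When its Box overlaps another actor, it applies a small fixed amount of damage, hides the projectile flipbook and halts ProjectileMovement with gravity zeroed.
; It then shows the hit flipbook as a non-looping effect and destroys itself after a short delay.
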(event `self.Box.OnComponentBeginOverlap`
  (params (OverlappedComponent :type "PrimitiveComponent Object Reference") (OtherActor :type "Actor Object Reference") (OtherComp :type "PrimitiveComponent Object Reference") (OtherBodyIndex :type Integer) (bFromSweep :type Boolean) (SweepResult :type "HitResult Structure (by ref)"))
  (bind _fbhit (`self.FbHit`))
  (bind _projectilemovement (`self.ProjectileMovement`))
  (if (!= OtherActor self)
    (`GameplayStatics.ApplyDamage` OtherActor 3.0)
    (`SceneComponent.SetVisibility` (`self.FbProjectTile`) false false)
    (set `ProjectileMovementComponent.ProjectileGravityScale` 0.0 _projectilemovement)
    (`MovementComponent.StopMovementImmediately` _projectilemovement)
    (`SceneComponent.SetVisibility` _fbhit true false)
    (`PaperFlipbookComponent.SetPlayRate` _fbhit 1.0)
    (`PaperFlipbookComponent.SetLooping` _fbhit false)
    (`KismetSystemLibrary.Delay` 0.35)
    (`self.K2_DestroyActor`)))

(fn `UserConstructionScript`)