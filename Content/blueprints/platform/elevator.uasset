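; Elevator platform Blueprint that raises its Cube when a BP_hero or BP_hero1 enters the Box trigger.
; Box overlap stores the actor's location and plays a Timeline, which lerps the Cube's Z up by 200 units.
; The stored world location is applied as the Cube's relative location.
; When either hero type leaves the Box, the Timeline reverses and lowers the Cube.
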(event `self.ReceiveBeginPlay`)

(event `self.Box.OnComponentBeginOverlap`
  (params (OverlappedComponent :type "PrimitiveComponent Object Reference") (OtherActor :type "Actor Object Reference") (OtherComp :type "PrimitiveComponent Object Reference") (OtherBodyIndex :type Integer) (bFromSweep :type Boolean) (SweepResult :type "HitResult Structure (by ref)"))
  (bind (_newvar_x _newvar_y _newvar_z) (`KismetMathLibrary.BreakVector` (`self.NewVar`)))
  (cast `/Game/blueprints/main_char/BP_hero` OtherActor
    (:`then`
      _)
    (:`CastFailed`
      (cast `/Game/blueprints/clon_char/BP_hero1` OtherActor)))
  (set `self.NewVar` (`self.K2_GetActorLocation`))
  (bind (_direction _newtrack_0) (`Timeline|Timeline` :!label _label)
    (:`Update`
      (`SceneComponent.K2_SetRelativeLocation` (`self.Cube`) (`KismetMathLibrary.MakeVector` _newvar_x _newvar_y (`KismetMathLibrary.Lerp` _newvar_z (+ _newvar_z 200.0) _newtrack_0)) false false))))

(event `self.Box.OnComponentEndOverlap`
  (params (OverlappedComponent :type "PrimitiveComponent Object Reference") (OtherActor :type "Actor Object Reference") (OtherComp :type "PrimitiveComponent Object Reference") (OtherBodyIndex :type Integer))
  (cast `/Game/blueprints/main_char/BP_hero` OtherActor
    (:`then`
      (goto _label :!via `Reverse`))
    (:`CastFailed`
      (cast `/Game/blueprints/clon_char/BP_hero1` OtherActor)
      (goto _label :!via `Reverse`))))

(fn `UserConstructionScript`)