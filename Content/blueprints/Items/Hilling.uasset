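; Healing pickup item that restores health to the player's BP_hero and then removes itself.
; On BeginPlay it caches the hero and plays the Moving timeline to animate the sprite's relative location.
; The first sphere overlap, with no check on the overlapping actor, adds HealingValue unclamped and sends the new health ratio to the hero.
; The Up timeline then moves the sprite, and the actor is destroyed after a short delay.
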(event `self.ReceiveBeginPlay`
  (bind _asbp_hero (cast `/Game/blueprints/main_char/BP_hero` (`GameplayStatics.GetPlayerCharacter` 0)))
  (set `self.BP Hero` _asbp_hero)
  (bind (_direction _newtrack_0) (`Timeline|Moving`)
    (:`Update`
      (`SceneComponent.K2_SetRelativeLocation` (`self.PaperSprite`) _newtrack_0 false false))))

(event `self.Sphere.OnComponentBeginOverlap`
  (params (OverlappedComponent :type "PrimitiveComponent Object Reference") (OtherActor :type "Actor Object Reference") (OtherComp :type "PrimitiveComponent Object Reference") (OtherBodyIndex :type Integer) (bFromSweep :type Boolean) (SweepResult :type "HitResult Structure (by ref)"))
  (bind _bp_hero (`self.BP Hero`))
  (bind _bp_hero_2 (`self.BP Hero`))
  (`/Engine/EditorBlueprintResources/StandardMacros.DoOnce` false
    (:`Completed`
      (set `/Game/blueprints/main_char/BP_hero.Health` (+ (`/Game/blueprints/main_char/BP_hero.Health` _bp_hero) (`self.HealingValue`)) _bp_hero)
      (`/Game/blueprints/main_char/BP_hero.changeHealth` _bp_hero (/ (`/Game/blueprints/main_char/BP_hero.Health` _bp_hero_2) (`/Game/blueprints/main_char/BP_hero.MaxHealth` _bp_hero_2)))
      (bind (_direction _newtrack_0) (`Timeline|up`)
        (:`Update`
          (`SceneComponent.K2_SetRelativeLocation` (`self.PaperSprite`) _newtrack_0 false false)
          (`KismetSystemLibrary.Delay` 0.4)
          (`self.K2_DestroyActor`))))))

(fn `UserConstructionScript`)